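; AI controller for the Troll enemy that runs its behavior tree and tracks whether it can see the player.
; On possession it starts the BT_AITroll behavior tree.
; AI perception updates filter for actors tagged Player and write the sensing result to the PlayerVisible blackboard key for the tree to use.
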(event `self.ReceivePossess`
  (params (PossessedPawn :type "Pawn Object Reference"))
  (`parent.ReceivePossess` PossessedPawn)
  (`self.RunBehaviorTree` "/Game/Project/AI/Troll/BT_AITroll.BT_AITroll"))

(event `self.AIPerception.OnTargetPerceptionUpdated`
  (params (Actor :type "Actor Object Reference") (Stimulus :type "AIStimulus Structure"))
  ;[1 1 1] Determine if the AI see the Player and update the corresponding variable
  (if (`self.ActorHasTag` Actor "Player")
    (if (`.bSuccessfullySensed` (break `AIStimulus` Stimulus))
      (`BlackboardComponent.SetValueAsBool` (`self.Blackboard`) "PlayerVisible" true)
      (else
        (`BlackboardComponent.SetValueAsBool` (`self.Blackboard`) "PlayerVisible" false)))))

(fn `UserConstructionScript`)