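; Minion AI controller that runs the Minion_BT behavior tree on possession and feeds its blackboard with what the minion perceives of the player.
; Sensing an actor tagged Player sets line of sight and the target actor, and cancels any pending loss timer.
; Losing the player stores their last location and starts a LineOfSightTimer delay, after which line of sight and target are cleared.
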(event `self.ReceivePossess`
  (params (PossessedPawn :type "Pawn Object Reference"))
  ;[1 1 1] Set up JustLoseSight
  (`self.RunBehaviorTree` "/Game/Project/AI/Minions/Minion_BT.Minion_BT")
  (`BlackboardComponent.SetValueAsBool` (`self.Blackboard`) "JustLoseSight" true))

(event `self.AIPerception.OnTargetPerceptionUpdated`
  (params (Actor :type "Actor Object Reference") (Stimulus :type "AIStimulus Structure"))
  (bind _blackboard (`self.Blackboard`))
  ;[1 1 1] Determine if the AI see the Player and update the corresponding variable
  (if (`self.ActorHasTag` Actor "Player")
    (if (`.bSuccessfullySensed` (break `AIStimulus` Stimulus))
      (`KismetSystemLibrary.K2_ClearAndInvalidateTimerHandle` (`self.EnemyTimer`))
      (`BlackboardComponent.SetValueAsBool` _blackboard "HasLineOfSight" true)
      (`BlackboardComponent.SetValueAsObject` _blackboard "PlayerActor" Actor)
      (else
        (bind _returnvalue (`KismetSystemLibrary.K2_SetTimerDelegate` (delegate `StartEnemyTimer`) (`self.LineOfSightTimer`)))
        (set `self.EnemyTimer` _returnvalue)
        (`BlackboardComponent.SetValueAsVector` _blackboard "PlayerLastLocation" (`self.K2_GetActorLocation` Actor))))))

(event `StartEnemyTimer`
  (bind _blackboard (`self.Blackboard`))
  ;[1 1 1] Determine if the AI see the Player and update the corresponding variable
  (`BlackboardComponent.SetValueAsBool` _blackboard "HasLineOfSight" false)
  (`BlackboardComponent.SetValueAsObject` _blackboard "PlayerActor" null))

(fn `UserConstructionScript`)