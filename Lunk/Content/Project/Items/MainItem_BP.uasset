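; Base pickup item that the Wukong player character can collect when nearby and within a vision-cone check.
; A detection sphere tracks overlap, and Tick runs the cone check while in range to set CanCollect and toggle a world-space name widget.
; The player's collect dispatcher calls TryCollect, which passes the item to PickUpItem when collectable.
; Logic to offset the widget above the mesh bounds exists but never runs.
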(event `self.ReceiveBeginPlay`
  (bind _lunkcharacter (`/Game/Project/BPFL.GetPlayer`))
  (add `/Game/Project/Characters/Wukong_Character_BP.Dispatch_Collect` _lunkcharacter (delegate `TryCollect`))
  (bind _asui_item_name (cast `/Game/Project/Widget/UI_ItemName` (`WidgetComponent.GetUserWidgetObject` (`self.UI-ItemName(World)`))))
  (bind _output_get (set `self.UI_ItemName` _asui_item_name))
  (`Widget.SetVisibility` _output_get "Collapsed")
  (set `self.ItemNameDisplayed` false))

(event `TryCollect`
  (if (`self.CanCollect`)
    (bind _lunkcharacter (`/Game/Project/BPFL.GetPlayer`))
    (`/Game/Project/Characters/Wukong_Character_BP.PickUp_Item` _lunkcharacter self)))

(event `self.ReceiveTick`
  (params (DeltaSeconds :type "Float (single-precision)"))
  (if (`self.IsInRange`)
    (bind _lunkcharacter (`/Game/Project/BPFL.GetPlayer`))
    (bind _incov (`/Game/Project/BPFL.IsInConeOfVision` _lunkcharacter (`self.K2_GetActorLocation`) (`self.COV_Angle`)))
    (if _incov
      (set `self.CanCollect` true)
      (`self.Display_ItemName`)
      (else
        (set `self.CanCollect` false)
        (`self.Remove_ItemName`)))
    (else
      (set `self.CanCollect` false)
      (`self.Remove_ItemName`))))

(event `self.DetectionSphere.OnComponentBeginOverlap`
  (params (OverlappedComponent :type "PrimitiveComponent Object Reference") (OtherActor :type "Actor Object Reference") (OtherComp :type "PrimitiveComponent Object Reference") (OtherBodyIndex :type Integer) (bFromSweep :type Boolean) (SweepResult :type "HitResult Structure (by ref)"))
  (cast `/Game/Project/Characters/Wukong_Character_BP` OtherActor)
  (set `self.IsInRange` true))

(event `self.DetectionSphere.OnComponentEndOverlap`
  (params (OverlappedComponent :type "PrimitiveComponent Object Reference") (OtherActor :type "Actor Object Reference") (OtherComp :type "PrimitiveComponent Object Reference") (OtherBodyIndex :type Integer))
  (cast `/Game/Project/Characters/Wukong_Character_BP` OtherActor)
  (set `self.IsInRange` false))

(fn `Display_ItemName`
  (if (not (`self.ItemNameDisplayed`))
    (`Widget.SetVisibility` (`self.UI_ItemName`) "Visible")
    (set `self.ItemNameDisplayed` true)))

(fn `Remove_ItemName`
  (if (`self.ItemNameDisplayed`)
    (`Widget.SetVisibility` (`self.UI_ItemName`) "Collapsed")
    (set `self.ItemNameDisplayed` false)))

(fn `UserConstructionScript`)