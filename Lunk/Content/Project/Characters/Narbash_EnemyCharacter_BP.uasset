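; Enemy character Blueprint for Narbash, with hit points and an HP bar widget.
; On BeginPlay it passes itself to the UI_HPBar widget in its HPUI component as the linked character.
; Tick polls HP and destroys the actor once it reaches zero or below.
; A helper function sets the movement component's max walk speed.
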(event `self.ReceiveTick`
  (params (DeltaSeconds :type "Float (single-precision)"))
  (`parent.ReceiveTick` 0.0)
  (if (<= (`self.HP`) 0)
    (`self.K2_DestroyActor`)))

(event `self.ReceiveBeginPlay`
  (`parent.ReceiveBeginPlay`)
  ;[1 1 1] Bind character to hp bar
  (bind _asui_hpbar (cast `/Game/Project/Widget/UI_HPBar` (`WidgetComponent.GetUserWidgetObject` (`self.HP_UI`))))
  (set `/Game/Project/Widget/UI_HPBar.CharacterLinked` self _asui_hpbar))

(fn `UpdateWalkSpeed`
  (params (NewWalkSpeed :type "Float (double-precision)"))
  (set `CharacterMovementComponent.MaxWalkSpeed` NewWalkSpeed (`self.CharacterMovement`)))

(fn `UserConstructionScript`)