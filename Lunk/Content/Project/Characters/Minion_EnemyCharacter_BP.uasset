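; Minion enemy character, spawned under a troll owner, with an HP bar widget.
; On BeginPlay it links itself to the HP bar on its widget component.
; Each tick it checks HP; at zero or below it decrements the troll owner's in-game minion count and destroys itself.
; A helper function sets its max walk speed on the movement component.
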(event `self.ReceiveTick`
  (params (DeltaSeconds :type "Float (single-precision)"))
  (bind _trollowner (`self.TrollOwner`))
  (`|ExecutionSequence`
    (:`then_0`
      (if (<= (`self.HP`) 0)
        (set `/Game/Project/Characters/Troll_EnemyCharacter_BP.MinionsNumberInGame` (- (`/Game/Project/Characters/Troll_EnemyCharacter_BP.MinionsNumberInGame` _trollowner) 1) _trollowner)
        (`self.K2_DestroyActor`)))
    (:`then_1`
      (`parent.ReceiveTick` DeltaSeconds))))

(event `self.ReceiveBeginPlay`
  (`parent.ReceiveBeginPlay`)
  ;[1 1 1] Bind character to hp bar
  (bind _asui_hpbar (cast `/Game/Project/Widget/UI_HPBar` (`WidgetComponent.GetUserWidgetObject` (`self.HP_UI`))))
  (set `/Game/Project/Widget/UI_HPBar.CharacterLinked` self _asui_hpbar))

(fn `UpdateWalkSpeed`
  (params (NewWalkSpeed :type "Float (double-precision)"))
  (set `CharacterMovementComponent.MaxWalkSpeed` NewWalkSpeed (`self.CharacterMovement`)))

(fn `UserConstructionScript`)