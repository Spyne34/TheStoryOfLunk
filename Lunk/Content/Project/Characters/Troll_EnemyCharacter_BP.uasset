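; Troll enemy character that tracks its distance to the player, can spawn minions and destroys itself when HP runs out.
; BeginPlay links it to its HP bar widget.
; Each tick sets aggro, CAC, AOE and range zone flags from 2D player distance.
; SpawnMinions, not called within this Blueprint, places a random count of owner-linked minions at reachable nearby points, up to a live-count cap.
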(event `self.ReceiveBeginPlay`
  (`parent.ReceiveBeginPlay`)
  ;[1 1 1] Bind character to hp bar
  (bind _asui_hpbar (cast `/Game/Project/Widget/UI_HPBar` (`WidgetComponent.GetUserWidgetObject` (`self.HP_UI`))))
  (set `/Game/Project/Widget/UI_HPBar.CharacterLinked` self _asui_hpbar))

(event `self.ReceiveTick`
  (params (DeltaSeconds :type "Float (single-precision)"))
  (`parent.ReceiveTick` DeltaSeconds)
  (`self.UpdateZones`)
  (`|ExecutionSequence`
    (:`then_0`
      (if (<= (`self.HP`) 0)
        (`self.K2_DestroyActor`)))))

(fn `SpawnMinions`
  (params (SpawnRadius :type "Float (double-precision)" :default 5000.0) (MinMob :type "Float (double-precision)" :default 3.0) (MaxMob :type "Float (double-precision)" :default 5.0))
  (for _ (range (`KismetMathLibrary.FTrunc` (`KismetMathLibrary.RandomFloatInRange` MinMob MaxMob)))
    (if (< (`self.MinionsNumberInGame`) (`self.MaxMinionsSpawned`))
      (bind _returnvalue (`|SpawnActorFromClass` "/Game/Project/Characters/Minion_EnemyCharacter_BP.Minion_EnemyCharacter_BP_C" (`KismetMathLibrary.MakeTransform` (`NavigationSystemV1.K2_GetRandomReachablePointInRadius` (`self.K2_GetActorLocation`) SpawnRadius null null)) "AdjustIfPossibleButAlwaysSpawn" "OverrideRootScale" null null))
      (set `/Game/Project/Characters/Minion_EnemyCharacter_BP.TrollOwner` self _returnvalue)
      (set `self.MinionsNumberInGame` (+ (`self.MinionsNumberInGame`) 1)))))

(fn `UpdateZones`
  (locals (Distance :type "Float (double-precision)"))
  (`|ExecutionSequence`
    (:`then_0`
      (bind _lunkcharacter (`/Game/Project/BPFL.GetPlayer`))
      (set `local.Distance` (`KismetMathLibrary.Vector_Distance2D` (`self.K2_GetActorLocation` _lunkcharacter) (`self.K2_GetActorLocation`))))
    (:`then_1`
      (set `self.InAggroZone` (<= (`local.Distance`) (`self.AggroRadius`)))
      (set `self.InCacZone` (<= (`local.Distance`) (`self.CacRadius`)))
      (set `self.InAoeZone` (<= (`local.Distance`) (`self.AoeRadius`)))
      (set `self.InRangeZone` (<= (`local.Distance`) (`self.RangeRadius`))))))

(fn `UserConstructionScript`
  (`parent.UserConstructionScript`))