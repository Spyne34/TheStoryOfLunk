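; Player heal skill Blueprint that restores health to the Wukong character.
; On an execution request, it plays the heal montage on the owning character and on its WukongFuryFX skeletal mesh.
; The separate execute event calls the character's Heal function with HealAmount.
; Both events require a valid owner that casts to Wukong_Character_BP.
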(event `self.Event_OnRequestExecutionBP`
  (bind _characterowner (`self.CharacterOwner`))
  ;[1 1 1] Play Animation
  (if (`KismetSystemLibrary.IsValid` _characterowner)
    (bind _aswukong_character_bp (cast `/Game/Project/Characters/Wukong_Character_BP` _characterowner))
    (`Character.PlayAnimMontage` _characterowner "/Game/Project/Animation/Heal_Wukong_Montage.Heal_Wukong_Montage" 1.0 "None")
    (`|PlayMontage` (`/Game/Project/Characters/Wukong_Character_BP.Wukong_Fury_FX` _aswukong_character_bp) "/Game/Project/Animation/Heal_Wukong_Montage.Heal_Wukong_Montage")))

(event `self.Event_OnExecuteBP`
  (bind _characterowner (`self.CharacterOwner`))
  ;[1 1 1] Heal the Player
  (if (`KismetSystemLibrary.IsValid` _characterowner)
    (bind _aswukong_character_bp (cast `/Game/Project/Characters/Wukong_Character_BP` _characterowner))
    (`/Game/Project/Characters/ThirdPersonCharacter_BP.Heal` _aswukong_character_bp (`self.HealAmount`))))