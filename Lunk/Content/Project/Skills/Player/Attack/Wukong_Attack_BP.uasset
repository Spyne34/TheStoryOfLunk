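; Wukong player attack skill that damages troll enemies hit by its detection mesh.
; On begin overlap, it checks for a valid owner, casts the other actor to the troll enemy class and skips the owner itself.
; The Wukong owner converts the skill's base Damage through GetFinalDamage, and the result is passed to the troll's TakeDamage.
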(event `self.Event_DetectionMeshBeginOverlapBP`
  (params (OverlappedComponent :type "PrimitiveComponent Object Reference") (OtherActor :type "Actor Object Reference") (OtherComp :type "PrimitiveComponent Object Reference") (OtherBodyIndex :type Integer) (bFromSweep :type Boolean) (SweepResult :type "HitResult Structure (by ref)"))
  (bind _characterowner (`self.CharacterOwner`))
  ;[1 1 1] Make the damage
  (if (`KismetSystemLibrary.IsValid` _characterowner)
    (bind _astroll_enemy_character_bp (cast `/Game/Project/Characters/Troll_EnemyCharacter_BP` OtherActor))
    (if (!= _astroll_enemy_character_bp _characterowner)
      (bind _aswukong_character_bp (cast `/Game/Project/Characters/Wukong_Character_BP` (`self.CharacterOwner`)))
      (bind _finaldamage (`/Game/Project/Characters/Wukong_Character_BP.GetFinalDamage` _aswukong_character_bp (`self.damage`)))
      (`/Game/Project/Characters/ThirdPersonCharacter_BP.TakeDamage` _astroll_enemy_character_bp _finaldamage))))