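; Old enemy melee attack skill for the Narbash enemy character, used against the Wukong character.
; On an execution request, it plays the melee attack montage on the owning Narbash character.
; When the detection mesh begins overlapping a Wukong character other than the owner, it passes the skill's damage, truncated to an integer, to that character's TakeDamage.
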(event `self.Event_OnRequestExecutionBP`
  (bind _characterowner (`self.CharacterOwner`))
  ;[1 1 1] Play Animation
  (if (`KismetSystemLibrary.IsValid` _characterowner)
    (bind _asnarbash_enemy_character_bp (cast `/Game/Project/Characters/Narbash_EnemyCharacter_BP` _characterowner))
    (`Character.PlayAnimMontage` _asnarbash_enemy_character_bp "/Game/Project/Animation/MeleeAttack_Enemy_Montage.MeleeAttack_Enemy_Montage" 1.0 "None")))

(event `self.Event_DetectionMeshBeginOverlapBP`
  (params (OverlappedComponent :type "PrimitiveComponent Object Reference") (OtherActor :type "Actor Object Reference") (OtherComp :type "PrimitiveComponent Object Reference") (OtherBodyIndex :type Integer) (bFromSweep :type Boolean) (SweepResult :type "HitResult Structure (by ref)"))
  (bind _characterowner (`self.CharacterOwner`))
  ;[1 1 1] Make the damage
  (if (`KismetSystemLibrary.IsValid` _characterowner)
    (bind _aswukong_character_bp (cast `/Game/Project/Characters/Wukong_Character_BP` OtherActor))
    (if (!= _aswukong_character_bp _characterowner)
      (`/Game/Project/Characters/ThirdPersonCharacter_BP.TakeDamage` _aswukong_character_bp (`KismetMathLibrary.FTrunc` (`self.damage`))))))