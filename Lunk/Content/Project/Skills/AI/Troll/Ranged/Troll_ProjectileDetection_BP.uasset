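; Projectile actor for the troll's ranged attack, moving a fireball forward with a collision box.
; BeginPlay binds to the owning attack's collide dispatcher, spawns a tinted shockwave and starts a timeline that sets speed for Tick movement.
; Expired duration, polled by a delay loop, or reaching max range disables collision and deactivates the fireball before delayed destruction.
; The collide dispatch spawns hit effects and destroys it immediately.
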(event `self.ReceiveBeginPlay`
  (bind _projectilemesh (`self.projectileMesh`))
  ;[1 1 1] Bind Dispatch Collide
  (bind _astroll_ranged_attack_bp (cast `/Game/Project/Skills/AI/Troll/Ranged/Troll_RangedAttack_BP` (`self.skillOwner`)))
  (add `/Game/Project/Skills/AI/Troll/Ranged/Troll_RangedAttack_BP.DispatchCollide` _astroll_ranged_attack_bp (delegate `Collided`))
  ;[1 1 1] spawn shot shockwave
  (bind _returnvalue (`GameplayStatics.SpawnEmitterAtLocation` "/Game/FXVarietyPack/Particles/P_ky_shotShockwave.P_ky_shotShockwave" (`SceneComponent.K2_GetComponentLocation` _projectilemesh) (`SceneComponent.K2_GetComponentRotation` _projectilemesh)))
  (`ParticleSystemComponent.SetVectorParameter` _returnvalue "color" (`KismetMathLibrary.Conv_LinearColorToVector` (`self.color`)))
  ;[1 1 1] effect move correct
  (bind (_direction _valuecorrect) (`Timeline|Timeline_0`)
    (:`Update`
      (set `self.speedCorrect` _valuecorrect)
      ;[1 1 1] duration control
      (`KismetSystemLibrary.Delay` 0.1 :!label _label)
      (if (< (`self.duration`) 0.0)
        ;[1 1 1] fx deactivate
        (`PrimitiveComponent.SetCollisionEnabled` (`self.Box`) "NoCollision" :!label _label_2)
        (`ActorComponent.Deactivate` (`self.FireBall`))
        (`KismetSystemLibrary.Delay` 1.0)
        ;[1 1 1] effect destroy
        (`self.K2_DestroyActor`)
        (else
          (goto _label))))))

(event `self.ReceiveTick`
  (params (DeltaSeconds :type "Float (single-precision)"))
  ;[1 1 1] duration increment for control
  (`|ExecutionSequence`
    (:`then_0`
      (set `self.duration` (- (`self.duration`) DeltaSeconds))
      ;[1 1 1] move control
      (`self.K2_AddActorLocalOffset` (`KismetMathLibrary.MakeVector` (* (`self.speedCorrect`) (`GameplayStatics.GetWorldDeltaSeconds`)))))
    (:`then_1`
      ;[1 1 1] Max Range Check
      (if (>= (`self.distanceTravelled`) (`self.maxRange`))
        (goto _label_2)))))

(event `Collided`
  ;[1 1 1] spawn collison fx
  (`GameplayStatics.SpawnEmitterAtLocation` (`self.hitFx`) (`SceneComponent.K2_GetComponentLocation` (`self.Box`)))
  ;[1 1 1] fx destroy
  (`self.K2_DestroyActor`))

(fn `UserConstructionScript`)