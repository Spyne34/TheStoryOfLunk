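; Troll ranged attack projectile Blueprint that damages the Wukong player character on overlap.
; The overlap event requires a valid owner and target, and ignores actors tagged as troll fireballs.
; A Wukong character takes the projectile's damage before the collide dispatch is called.
; Any other untagged actor triggers only the collide dispatch, without damage.
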(event `self.Event_ProjectileBeginOverlapBP`
  (params (OverlappedComponent :type "PrimitiveComponent Object Reference") (OtherActor :type "Actor Object Reference") (OtherComp :type "PrimitiveComponent Object Reference") (OtherBodyIndex :type Integer) (bFromSweep :type Boolean) (SweepResult :type "HitResult Structure (by ref)"))
  ;[1 1 1] Collision and Damage
  (if (`KismetSystemLibrary.IsValid` (`self.CharacterOwner`))
    (if (`KismetSystemLibrary.IsValid` OtherActor)
      (if (not (`Actor.ActorHasTag` OtherActor "Troll_Fireball"))
        (bind _aswukong_character_bp (cast `/Game/Project/Characters/Wukong_Character_BP` OtherActor)
          (:`then`
            (`/Game/Project/Characters/ThirdPersonCharacter_BP.TakeDamage` _aswukong_character_bp (`self.damage`))
            (`self.DispatchCollide`))
          (:`CastFailed`
            (`self.DispatchCollide`)))))))